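; BP_PushingWall is a wall actor that moves along a set path when a ball enters its trigger box.
; An overlap by an actor tagged Ball plays a timeline that lerps the actor's relative location between StartPoint and EndPoint without sweep.
; A CanTrigger flag blocks retriggering until the timeline finishes.
; The construction script applies the configurable WallMaterial to the wall mesh.
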(event `self.TriggerBox.OnComponentBeginOverlap`
  (params (OverlappedComponent :type "PrimitiveComponent Object Reference") (OtherActor :type "Actor Object Reference") (OtherComp :type "PrimitiveComponent Object Reference") (OtherBodyIndex :type Integer) (bFromSweep :type Boolean) (SweepResult :type "HitResult Structure (by ref)"))
  (if (and (`self.CanTrigger`) (`self.ActorHasTag` OtherActor "Ball"))
    (set `self.CanTrigger` false)
    (bind (_direction _float_track) (`Timeline|Timeline` :!via `PlayFromStart`)
      (:`Update`
        (`self.K2_SetActorRelativeLocation` (`KismetMathLibrary.VLerp` (`self.StartPoint`) (`self.EndPoint`) _float_track)))
      (:`Finished`
        (set `self.CanTrigger` true)))))

(fn `UserConstructionScript`
  (`PrimitiveComponent.SetMaterial` (`self.WallMesh`) 0 (`self.WallMaterial`)))